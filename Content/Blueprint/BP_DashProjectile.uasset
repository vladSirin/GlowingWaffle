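; BP_DashProjectile is a projectile that teleports its instigator to the point where it explodes.
; It overrides hit and overlap events with empty bodies and instead sets a timer at BeginPlay to explode.
; Explode runs the parent behavior, stores the location and starts a short second timer for the teleport.
; The teleport keeps the instigator's control rotation, then destroys the projectile and prints a message if it failed.
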(event Custom|Teleport
  (bind _returnvalue (Game|GetInstigator))
  ;[1 1 1] Teleport
  (if (Utilities|IsValid _returnvalue)
    (bind _returnvalue_2 (Transformation|Teleport _returnvalue (Variables|Default|GetTeleportLocation) (Pawn|GetControlRotation _returnvalue :!class /Script/Engine.Pawn)))
    (Utilities|FlowControl|Sequence
      (:then_0
        (Actor|DestroyActor))
      (:then_1
        (if (not _returnvalue_2)
          (Development|PrintString "Position Invalid!"))))))

(event EventBeginPlay
  ;[1 1 1] Explode after X secs
  (Utilities|Time|SetTimerbyEvent (delegate EventExplode) 1.0))

(event EventExplode
  ;[1 1 1] Teleport after X secs when Explode
  (|CallParentFunction)
  (Variables|Default|SetTeleportLocation (Transformation|GetActorLocation))
  (Utilities|Time|SetTimerbyEvent (delegate Custom|Teleport) 0.2))

(event EventOnHit
  (params (HitComponent :type Primitive%20Component%20Object%20Reference) (OtherActor :type Actor%20Object%20Reference) (OtherComp :type Primitive%20Component%20Object%20Reference) (NormalImpulse :type Vector :default "0, 0, 0") (Hit :type Hit%20Result%20Structure%20%28by%20ref%29))
  ;[1 1 1] Override
)

(event EventOnOverlap
  (params (OverlappedComponent :type Primitive%20Component%20Object%20Reference) (OtherActor :type Actor%20Object%20Reference) (OtherComp :type Primitive%20Component%20Object%20Reference) (OtherBodyIndex :type Integer) (bFromSweep :type Boolean) (SweepResult :type Hit%20Result%20Structure%20%28by%20ref%29))
  ;[1 1 1] Override
)

(fn ConstructionScript)