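; BP_PickupSpawnMarker is a marker actor that spawns one random pickup, either a coin or a health potion, at an EQS-chosen location.
; On BeginPlay it runs the EQS_FindPickUpPoint query with itself as querier, picking randomly from the best 25% of points.
; When the query finishes with valid locations, it spawns the pickup at a random returned point, raised above it, ignoring collisions.
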(event Custom|OnQueryFinished
  (params (QueryInstance :type Env%20Query%20Instance%20Blueprint%20Wrapper%20Object%20Reference) (QueryStatus :type EEnvQueryStatus%20Enum :default "Processing"))
  (bind (_resultlocations _returnvalue) (AI|EQS|GetQueryResultsasLocations QueryInstance))
  (if _returnvalue
    (Game|SpawnActorfromClass (Utilities|Select :Index (Math|Random|RandomInteger 2) :Option%200 "/Game/Blueprint/BP_CoinPickup.BP_CoinPickup_C" :Option%201 "/Game/Blueprint/BP_HealthPotion.BP_HealthPotion_C") (Math|Conversions|ToTransform(Vector) (Math|Vector|MakeVector (.X (Class|KismetMathLibrary|BreakVector3f (.OutItem (Utilities|Array|Random _resultlocations)))) (.Y (Class|KismetMathLibrary|BreakVector3f (.OutItem (Utilities|Array|Random _resultlocations)))) (+ (.Z (Class|KismetMathLibrary|BreakVector3f (.OutItem (Utilities|Array|Random _resultlocations)))) 9e+01))) "AlwaysSpawn" 0)))

(event EventBeginPlay
  (bind _returnvalue (AI|EQS|RunEQSQuery "/Game/AI/EQS_FindPickUpPoint.EQS_FindPickUpPoint" self "RandomBest25Pct"))
  (EventDispatchers|BindEventtoOnQueryFinishedEvent _returnvalue (delegate Custom|OnQueryFinished)))

(fn ConstructionScript)