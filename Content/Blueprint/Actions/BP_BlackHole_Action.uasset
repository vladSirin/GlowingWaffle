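; Black hole action that costs Rage to use, layered on a parent action class.
; CanStart requires both the parent's check to pass and the instigator's attributes to hold at least RageCost in Rage.
; StartAction consumes that Rage from the instigator, then hands off to the parent's start logic, as no black hole behavior is defined in these graphs.
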(event EventStartAction
  (params (Instigator :type Actor%20Object%20Reference))
  (Class|WaffGameplayFunctionLibrary|ConsumeRage Instigator Instigator (Variables|Default|GetRageCost))
  (|CallParentFunction Instigator))

(fn CanStart
  (params (Instigator :type Actor%20Object%20Reference))
  (bind _returnvalue (|CallParentFunction Instigator))
  (bind _returnvalue_2 (Class|WaffAttributeComponent|GetAttributes Instigator))
  (return (and _returnvalue (>= (Variables|/Script/GlowingWaffle.WaffAttributeComponent|GetRage _returnvalue_2) (Variables|Default|GetRageCost)))))