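; BP_BonFire is an interactable bonfire that acts as a world save point.
; Interacting sets FireActive, then asks BP_WaffGameMode to write the save game and prints a confirmation before refreshing the flame.
; UpdateFlame activates the particle system when FireActive is set, and also runs on OnActorLoaded to restore a lit fire after loading.
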(event Custom|UpdateFlame
  (if (Variables|Default|GetbFireActive)
    (Components|Activation|Activate (Variables|Default|GetParticleSystem) false)))

(event EventBeginPlay)

(event Collision|EventActorBeginOverlap
  (params (OtherActor :type Actor%20Object%20Reference)))

(event EventTick
  (params (DeltaSeconds :type Float%20%28single-precision%29)))

(event EventInteract
  (params (InstigatorPawn :type Pawn%20Object%20Reference))
  (Variables|Default|SetbFireActive true)
  (bind _asbp_waff_game_mode (Utilities|Casting|CastToBP_WaffGameMode (Game|GetGameMode)))
  (Class|GlowingWaffleGameModeBase|WriteSaveGame _asbp_waff_game_mode)
  (Development|PrintString "WORLD SAVED!")
  (CallFunction|UpdateFlame))

(event EventOnActorLoaded
  (CallFunction|UpdateFlame))

(fn ConstructionScript)